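; BP_Radio is a radio actor that switches on when another actor overlaps it, making a noise that AI hearing can pick up.
; The first overlap activates its Audio component and reports a single noise event at the radio's location, with itself as instigator.
; A delay deactivates the audio after 30 seconds.
; The Active flag is never cleared, so the radio triggers only once.
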(event EventBeginPlay)

(event Collision|EventActorBeginOverlap
  (params (OtherActor :type Actor%20Object%20Reference))
  (if (not (Variables|Default|GetActive))
    (Components|Activation|Activate (Variables|Default|GetAudio) false)
    (Variables|Default|SetActive true)
    (Class|AISenseHearing|ReportNoiseEvent (Transformation|GetActorLocation) 1.0 self 0.0 "None")
    (Utilities|FlowControl|Delay 3e+01)
    (Components|Activation|Deactivate (Variables|Default|GetAudio))))

(fn ConstructionScript)