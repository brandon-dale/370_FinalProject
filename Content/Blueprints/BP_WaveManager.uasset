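; Wave manager actor that runs zombie waves, started by interaction or box overlap when none is active.
; At BeginPlay it sorts tagged TargetPoints into enemy and item spawn lists.
; WaveStart randomly draws non-repeating points from copied lists to spawn zombies plus ammo, health and cash pickups.
; ZombieKilled counts down survivors; at zero, it ends the wave, enlarges the next and credits the player a kill and points.
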(event OnComponentBeginOverlap(BoxCollision)
  (params (OverlappedComponent :type Primitive%20Component%20Object%20Reference) (OtherActor :type Actor%20Object%20Reference) (OtherComp :type Primitive%20Component%20Object%20Reference) (OtherBodyIndex :type Integer) (bFromSweep :type Boolean) (SweepResult :type Hit%20Result%20Structure%20%28by%20ref%29))
  (CallFunction|WaveStart))

(event EventBeginPlay
  ;[1 1 1] Begin Play
  (bind _outactors (Actor|GetAllActorsOfClass "/Script/Engine.TargetPoint"))
  (for _array_element _outactors
    (if (Actor|ActorHasTag _array_element "ItemSpawn")
      (Utilities|Array|Add (Variables|Default|GetOrigItemLocations) _array_element)
      (elif (Actor|ActorHasTag _array_element "EnemySpawn")
        (Utilities|Array|Add (Variables|Default|GetOrigEnemyLocations) _array_element)))))

(event EventInteract
  (CallFunction|WaveStart))

(fn ConstructionScript)

(fn WaveStart
  (if (not (Variables|Default|GetWaveActive)) ; only start if a wave is not active
    (Variables|Default|SetWaveActive true)
    (Math|Integer|IncrementInt (Variables|Default|GetWaveNumber)
      (:%20%20
        (Variables|Default|SetTempItemLocations (Variables|Default|GetOrigItemLocations)) ; Copy item spawn locs
        (Variables|Default|SetTempSpawnPoints (Variables|Default|GetOrigEnemyLocations)) ; Copy enemy spawn locs
        ;[1 1 1] Spawn Enemies
        (Utilities|FlowControl|ForLoopwithBreak 0 (Variables|Default|GetZombiesInWave) :!label _label
          (:LoopBody
            (if (> (Utilities|Array|Length (Variables|Default|GetTempSpawnPoints)) 0)
              (Utilities|Array|Swap (Variables|Default|GetTempSpawnPoints) (Math|Random|RandomIntegerinRange 0 (- (Utilities|Array|Length (Variables|Default|GetTempSpawnPoints)) 1)) (- (Utilities|Array|Length (Variables|Default|GetTempSpawnPoints)) 1))
              (bind _returnvalue (Game|SpawnActorfromClass "/Game/Blueprints/Enemies/BP_BasicZombie.BP_BasicZombie_C" (Transformation|GetActorTransform (Utilities|Array|Get(acopy) (Variables|Default|GetTempSpawnPoints) (- (Utilities|Array|Length (Variables|Default|GetTempSpawnPoints)) 1))) "Undefined" 0 0))
              (Transformation|SetActorRotation _returnvalue (Math|Rotator|MakeRotator 0.0 0.0 (* (Math|Random|RandomFloat) 3.6e+02)))
              (Math|Integer|IncrementInt (Variables|Default|GetZombiesAlive)
                (:%20%20
                  (Utilities|Array|RemoveIndex (Variables|Default|GetTempSpawnPoints) (- (Utilities|Array|Length (Variables|Default|GetTempSpawnPoints)) 1))))
              (else
                (goto _label Break))))
          (:Completed
            ;[1 1 1] Spawn Ammo
            (Utilities|Array|Swap (Variables|Default|GetTempItemLocations) (Math|Random|RandomIntegerinRange 0 (- (Utilities|Array|Length (Variables|Default|GetTempItemLocations)) 1)) (- (Utilities|Array|Length (Variables|Default|GetTempItemLocations)) 1))
            (Game|SpawnActorfromClass "/Game/Blueprints/Pickups/Ammo.Ammo_C" (Transformation|GetActorTransform (Utilities|Array|Get(acopy) (Variables|Default|GetTempItemLocations) (- (Utilities|Array|Length (Variables|Default|GetTempItemLocations)) 1))) "Undefined" 0 0)
            (Utilities|Array|RemoveIndex (Variables|Default|GetTempItemLocations) (- (Utilities|Array|Length (Variables|Default|GetTempItemLocations)) 1))
            ;[1 1 1] Spawn Health
            (Utilities|Array|Swap (Variables|Default|GetTempItemLocations) (Math|Random|RandomIntegerinRange 0 (- (Utilities|Array|Length (Variables|Default|GetTempItemLocations)) 1)) (- (Utilities|Array|Length (Variables|Default|GetTempItemLocations)) 1))
            (Game|SpawnActorfromClass "/Game/Blueprints/Pickups/HealthPickups.HealthPickups_C" (Transformation|GetActorTransform (Utilities|Array|Get(acopy) (Variables|Default|GetTempItemLocations) (- (Utilities|Array|Length (Variables|Default|GetTempItemLocations)) 1))) "Undefined" 0 0)
            (Utilities|Array|RemoveIndex (Variables|Default|GetTempItemLocations) (- (Utilities|Array|Length (Variables|Default|GetTempItemLocations)) 1))
            ;[1 1 1] Spawn Cash
            (Utilities|Array|Swap (Variables|Default|GetTempItemLocations) (Math|Random|RandomIntegerinRange 0 (- (Utilities|Array|Length (Variables|Default|GetTempItemLocations)) 1)) (- (Utilities|Array|Length (Variables|Default|GetTempItemLocations)) 1))
            (Game|SpawnActorfromClass "/Game/Blueprints/Pickups/CashDrop.CashDrop_C" (Transformation|GetActorTransform (Utilities|Array|Get(acopy) (Variables|Default|GetTempItemLocations) (- (Utilities|Array|Length (Variables|Default|GetTempItemLocations)) 1))) "Undefined" 0 0)
            (Utilities|Array|RemoveIndex (Variables|Default|GetTempItemLocations) (- (Utilities|Array|Length (Variables|Default|GetTempItemLocations)) 1))))))))

(fn ZombieKilled
  (bind _result (Math|Integer|DecrementInt (Variables|Default|GetZombiesAlive))
    (:%20%20
      (if (<= _result 0)
        (CallFunction|WaveDone)
        (bind _asbp_first_person_character (Utilities|Casting|CastToBP_FirstPersonCharacter (Game|Player|GetPlayerPawn 0)))
        (Variables|/Game/FirstPerson/Blueprints/BP_FirstPersonCharacter.BP_FirstPersonCharacter_C|Setkills _asbp_first_person_character (+ (Variables|/Game/FirstPerson/Blueprints/BP_FirstPersonCharacter.BP_FirstPersonCharacter_C|Getkills _asbp_first_person_character) 1))
        (Variables|/Game/FirstPerson/Blueprints/BP_FirstPersonCharacter.BP_FirstPersonCharacter_C|Setpoints _asbp_first_person_character (+ (Variables|/Game/FirstPerson/Blueprints/BP_FirstPersonCharacter.BP_FirstPersonCharacter_C|Getpoints _asbp_first_person_character) 100))))))

(fn WaveDone
  (Variables|Default|SetWaveActive false)
  (Variables|Default|SetZombiesInWave (+ (Variables|Default|GetZombiesInWave) 5)))