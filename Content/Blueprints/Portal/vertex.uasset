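; Portal actor that teleports the player between the game area and the upgrade room.
; Capsule overlap plays an effect, waits briefly, then moves the player to the average location of actors tagged for the opposite area, flipping the character's UpgradeRoom flag and toggling rain.
; Tick keeps Idle active and, once Ison is set by a return trip, sets the effect's world location to the camera's forward vector.
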(event OnComponentBeginOverlap(Capsule)
  (params (OverlappedComponent :type Primitive%20Component%20Object%20Reference) (OtherActor :type Actor%20Object%20Reference) (OtherComp :type Primitive%20Component%20Object%20Reference) (OtherBodyIndex :type Integer) (bFromSweep :type Boolean) (SweepResult :type Hit%20Result%20Structure%20%28by%20ref%29))
  (bind _returnvalue (Game|Player|GetPlayerPawn 0))
  (bind _returnvalue_2 (Game|Player|GetPlayerPawn 0))
  (bind _effect (Variables|Default|Geteffect))
  (bind _character (Variables|Default|Getcharacter))
  (bind _character_2 (Variables|Default|Getcharacter))
  (bind _effect_2 (Variables|Default|Geteffect))
  (if (Variables|/Game/FirstPerson/Blueprints/BP_FirstPersonCharacter.BP_FirstPersonCharacter_C|GetUpgradeRoom (Variables|Default|Getcharacter))
    (Components|Activation|Activate (Variables|Default|Geteffect) false)
    (Transformation|SetRelativeLocation _effect (Math|Vector|GetForwardVector (Variables|/Script/FinalProject.FinalProjectCharacter|GetFirstPersonCameraComponent (Variables|Default|Getcharacter))) false false)
    (Variables|Default|Setison true)
    (Transformation|SetRelativeRotation _effect "0, 0,90.000000" false false)
    (Utilities|FlowControl|Delay 2.0)
    (bind _outactors (Actor|GetAllActorswithTag "Game"))
    (bind _returnvalue_3 (Class|GameplayStatics|GetActorArrayAverageLocation _outactors))
    (if (== OtherActor _returnvalue_2)
      (Development|PrintText "ENTERING PORTAL")
      (Transformation|SetActorLocation _returnvalue_2 _returnvalue_3 false false)
      (Variables|/Game/FirstPerson/Blueprints/BP_FirstPersonCharacter.BP_FirstPersonCharacter_C|SetUpgradeRoom _character false)
      (Components|Activation|Activate (Variables|/Game/FirstPerson/Blueprints/BP_FirstPersonCharacter.BP_FirstPersonCharacter_C|GetRain _character) false)
      (Components|Activation|Deactivate (Variables|Default|Geteffect)))
    (else
      (Components|Activation|Activate (Variables|Default|Geteffect) false)
      (Transformation|SetRelativeLocation _effect_2 (Math|Vector|GetForwardVector (Variables|/Script/FinalProject.FinalProjectCharacter|GetFirstPersonCameraComponent (Variables|Default|Getcharacter))) false false)
      (Transformation|SetRelativeRotation _effect_2 "0, 0,90.000000" false false)
      (Utilities|FlowControl|Delay 2.0)
      (bind _outactors_2 (Actor|GetAllActorswithTag "UpgradeRoom"))
      (bind _returnvalue_4 (Class|GameplayStatics|GetActorArrayAverageLocation _outactors_2))
      (if (== OtherActor _returnvalue)
        (Development|PrintText "ENTERING PORTAL")
        (Transformation|SetActorLocation _returnvalue _returnvalue_4 false false)
        (Variables|/Game/FirstPerson/Blueprints/BP_FirstPersonCharacter.BP_FirstPersonCharacter_C|SetUpgradeRoom _character_2 true)
        (Components|Activation|Deactivate (Variables|/Game/FirstPerson/Blueprints/BP_FirstPersonCharacter.BP_FirstPersonCharacter_C|GetRain _character_2))
        (Components|Activation|Deactivate (Variables|Default|Geteffect))))))

(event EventBeginPlay
  (Components|Activation|Activate (Variables|Default|Getbegin) false)
  (bind _asbp_first_person_character (Utilities|Casting|CastToBP_FirstPersonCharacter (Game|Player|GetPlayerPawn 0)))
  (Variables|Default|Setcharacter _asbp_first_person_character))

(event EventTick
  (params (DeltaSeconds :type Float%20%28single-precision%29))
  (Components|Activation|Activate (Variables|Default|Getidle) false)
  (if (Variables|Default|Getison)
    (Transformation|SetWorldLocation (Variables|Default|Geteffect) (Math|Vector|GetForwardVector (Variables|/Script/FinalProject.FinalProjectCharacter|GetFirstPersonCameraComponent (Variables|Default|Getcharacter))) false false)))

(fn ConstructionScript)