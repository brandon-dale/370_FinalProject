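; An upgrade-room light that switches between green and red, with a noise on each change, when the player's UpgradeRoom flag is set.
; It caches the first-person character on BeginPlay and polls the flag every Tick.
; After a short delay it shows red, then returns to green after a longer one.
; An Activated latch prevents repeats until the flag clears.
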(event EventBeginPlay
  (bind _asbp_first_person_character (Utilities|Casting|CastToBP_FirstPersonCharacter (Game|Player|GetPlayerPawn 0)))
  (Variables|Default|Setplayer _asbp_first_person_character))

(event Collision|EventActorBeginOverlap
  (params (OtherActor :type Actor%20Object%20Reference)))

(event EventTick
  (params (DeltaSeconds :type Float%20%28single-precision%29))
  (if (Variables|/Game/FirstPerson/Blueprints/BP_FirstPersonCharacter.BP_FirstPersonCharacter_C|GetUpgradeRoom (Variables|Default|Getplayer))
    (if (not (Variables|Default|Getactivated))
      (Utilities|FlowControl|Delay 2.0)
      (Rendering|SetVisibility (Variables|Default|Getgreen) false false)
      (Rendering|SetVisibility (Variables|Default|Getred) true false)
      (Components|Activation|Activate (Variables|Default|Getlight_noise) false)
      (Variables|Default|Setactivated true)
      (Utilities|FlowControl|Delay 1e+01)
      (Rendering|SetVisibility (Variables|Default|Getred) false false)
      (Rendering|SetVisibility (Variables|Default|Getgreen) true false)
      (Components|Activation|Activate (Variables|Default|Getlight_noise) false))
    (else
      (Variables|Default|Setactivated false))))

(fn ConstructionScript)