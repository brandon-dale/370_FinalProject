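; Upgrade room light actor that makes three point lights flicker together at irregular intervals.
; Tick drives the loop through two chained random sub-second Delays, hiding the lights after the first and showing them after the second.
; Each Tick also calls Activate without reset on an Idle component ahead of the delays.
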(event EventBeginPlay)

(event Collision|EventActorBeginOverlap
  (params (OtherActor :type Actor%20Object%20Reference)))

(event EventTick
  (params (DeltaSeconds :type Float%20%28single-precision%29))
  (Components|Activation|Activate (Variables|Default|Getidle) false)
  (Utilities|FlowControl|Delay (Math|Random|RandomFloatinRange 0.0 1.0))
  (Rendering|SetVisibility (Variables|Default|GetPointLight) false false)
  (Rendering|SetVisibility (Variables|Default|GetPointLight1) false false)
  (Rendering|SetVisibility (Variables|Default|GetPointLight2) false false)
  (Utilities|FlowControl|Delay (Math|Random|RandomFloatinRange 0.0 1.0))
  (Rendering|SetVisibility (Variables|Default|GetPointLight) true false)
  (Rendering|SetVisibility (Variables|Default|GetPointLight1) true false)
  (Rendering|SetVisibility (Variables|Default|GetPointLight2) true false))

(fn ConstructionScript)