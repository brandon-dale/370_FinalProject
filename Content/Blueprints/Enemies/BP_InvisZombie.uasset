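; BP_InvisZombie is a wave-based zombie enemy that chases and attacks the player; its invisibility opacity logic is unconnected.
; Damage, death and player death write Blackboard keys for the behavior tree, with montages for hit, attack, scream and dying.
; A looping timer damages the player through IBP_TakeDamage, and a timeline turns wounded zombies toward targets.
; Death updates player kills and points, destroys the actor and notifies BP_WaveManager.
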(event Custom|Death
  ;[1 1 1] Death
  (AI|Components|Blackboard|SetValueasBool (AI|GetBlackboard 0) (Variables|Default|GetKey%20Name) true) ; Tell BT enemy is dead
  (Variables|Default|SetIsDead true)
  (bind _asbp_first_person_character (Utilities|Casting|CastToBP_FirstPersonCharacter (Game|Player|GetPlayerPawn 0)))
  (Default|UpdateKills _asbp_first_person_character)
  (Default|UpdatePoints _asbp_first_person_character)
  (bind _returnvalue (Animation|PlayAnimMontage "/Game/Blueprints/Enemies/Assets/Animations/zombie_dying_Montage.zombie_dying_Montage" 1.0 "None"))
  (Utilities|FlowControl|Delay (- _returnvalue 0.2))
  (Actor|DestroyActor)
  (bind _outactors (Actor|GetAllActorsOfClass "/Game/Blueprints/BP_WaveManager.BP_WaveManager_C")) ; Tell the wave manager that the zombie died
  (for _array_element _outactors
    (Default|ZombieKilled _array_element)))

(event Custom|Attack
  ;[1 1 1] Attack
  (if (Utilities|DoesObjectImplementInterface (Game|Player|GetPlayerPawn 0) "/Game/Blueprints/Interface/IBP_TakeDamage.IBP_TakeDamage_C")
    (CallFunction|TakeDamage (Variables|Default|GetDamage))))

(event Custom|Rotate%20Towards
  (params (Target%20Location :type Vector))
  ;[1 1 1] Rotate Towards
  (if (< (Variables|Default|GetHealth) 1e+02) ; Error check
    (bind _alpha (Timeline|Timeline_LerpValue PlayFromStart)
      (:Update
        (Transformation|SetActorRotation (Math|Rotator|Lerp(Rotator) (Transformation|GetWorldRotation (Variables|Collision|GetCapsuleComponent)) (Math|Rotator|FindLookatRotation (Transformation|GetActorLocation) Target%20Location) _alpha))))))

(event EventTakeDamage
  (params (Damage :type Float%20%28double-precision%29))
  (bind _returnvalue (AI|GetBlackboard 0))
  ;[1 1 1] Takes Damage
  (if (not (Variables|Default|GetIsDead))
    (bind _output_get (Variables|Default|SetHealth (- (Variables|Default|GetHealth) Damage))) ; Decrement Health By Damage
    (if (<= _output_get 0.0) ; If run out of health
      (CallFunction|Death)
      (else
        (Animation|Montage|PlayMontage (Variables|Character|GetMesh) "/Game/Blueprints/Enemies/Assets/Animations/Zombie_Reaction_Hit_mixamo_com_Montage.Zombie_Reaction_Hit_mixamo_com_Montage" ; Play zombie hit reaction animation
          (:then
            (AI|Components|Blackboard|SetValueasBool _returnvalue (Variables|Default|GetTookDamage) true)
            (AI|Components|Blackboard|SetValueasObject _returnvalue (Variables|Default|GetEnemyActor) (Game|Player|GetPlayerPawn 0))))))))

(event EventStopAI
  ;[1 1 1] Stop AI Interface Override
  (AI|Components|Blackboard|SetValueasBool (AI|GetBlackboard 0) (Utilities|Name|MakeLiteralName "PlayerDead") true))

(fn ConstructionScript)

(fn UpdateWalkSpeed
  (params (NewWalkSpeed :type Float%20%28double-precision%29))
  (Variables|/Script/Engine.CharacterMovementComponent|SetMaxWalkSpeed (Variables|Character|GetCharacterMovement) NewWalkSpeed))

(fn StartAttacking
  (Development|PrintString "Start Attacking")
  (bind _returnvalue (Utilities|Time|SetTimerbyFunctionName 0 (Variables|Default|GetDamagePlayer) (Variables|Default|GetAttackDuration) true (LocalVariables|GetAttackTimerStartDelay))) ; Start Attack Timer
  (Variables|Default|SetAttackTimerHandle _returnvalue) ; Save the timer handle
  (Animation|PlayAnimMontage "/Game/Blueprints/Enemies/Assets/Animations/zombie_attack_Montage1.zombie_attack_Montage1" 1.0 "None")
  (Audio|Components|Audio|Stop (Variables|Default|GetIdleSound))
  (Audio|Components|Audio|Play (Variables|Default|GetAttackSound) 0.0)
  (Audio|Components|Audio|Play (Variables|Default|GetChaseSound) 0.0))

(fn StopAttacking
  (Utilities|Time|ClearandInvalidateTimerbyHandle (Variables|Default|GetAttackTimerHandle)) ; Stop the attack timer
)

(fn DamagePlayer
  (bind _returnvalue (Game|Player|GetPlayerPawn 0))
  (Animation|PlayAnimMontage "/Game/Blueprints/Enemies/Assets/Animations/zombie_attack_Montage1.zombie_attack_Montage1" 1.0 "None")
  (if (Utilities|DoesObjectImplementInterface _returnvalue "/Game/Blueprints/Interface/IBP_TakeDamage.IBP_TakeDamage_C")
    (Class|IBPTakeDamage|TakeDamage(Message) _returnvalue (Variables|Default|GetDamage))
    (Development|PrintString "Damage Player")))

(fn Scream
  (Audio|Components|Audio|Stop (Variables|Default|GetIdleSound))
  (Audio|Components|Audio|Play (Variables|Default|GetScreamSound) 0.0)
  (bind _returnvalue (Animation|PlayAnimMontage "/Game/Blueprints/Enemies/Assets/Animations/zombie_scream_Montage.zombie_scream_Montage" 1.0 "None"))
  (return _returnvalue))

(fn StopAI
  (AI|Components|Blackboard|SetValueasBool (AI|GetBlackboard 0) (LocalVariables|GetPlayerDead) true))