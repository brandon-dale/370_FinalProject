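; Behavior tree task that checks whether the player is within a basic zombie's attack range.
; It compares the distance between the zombie and player pawn 0 against the zombie's Range variable.
; Out of range, it clears the IsAttacking blackboard value without calling FinishExecute.
; In range it finishes successfully, and a pawn that is not a BP_BasicZombie fails the task.
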(event EventReceiveExecuteAI
  (params (OwnerController :type AI%20Controller%20Object%20Reference) (ControlledPawn :type Pawn%20Object%20Reference))
  (bind _asbp_basic_zombie (Utilities|Casting|CastToBP_BasicZombie ControlledPawn)
    (:then
      (if (< (Variables|/Game/Blueprints/Enemies/BP_BasicZombie.BP_BasicZombie_C|GetRange _asbp_basic_zombie) (Math|Vector|Distance(Vector) (Transformation|GetActorLocation _asbp_basic_zombie) (Transformation|GetActorLocation (Game|Player|GetPlayerPawn 0)))) ; range < dist
        (AI|Components|Blackboard|SetValueasBool (AI|GetBlackboard ControlledPawn) (Variables|Default|GetIsAttacking) false) ; Set IsAttacking to false
        (else
          (AI|BehaviorTree|FinishExecute true))))
    (:CastFailed
      (AI|BehaviorTree|FinishExecute false))))