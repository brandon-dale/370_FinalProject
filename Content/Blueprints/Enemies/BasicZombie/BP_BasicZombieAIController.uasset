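; AI controller for the basic zombie that runs its behavior tree on possession and feeds perception results into the Blackboard.
; Sighting an actor with the required tag sets line of sight and the enemy actor, cancelling any pending lose-target timer.
; Other sight updates start a timer that clears both keys after a delay.
; Heard noises write their location to the PatrolLocation key, redirecting the zombie toward the sound.
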(event OnTargetPerceptionUpdated(AIPerception)
  (params (Actor :type Actor%20Object%20Reference) (Stimulus :type AI%20Stimulus%20Structure))
  (bind _blackboard (Variables|Default|GetBlackboard))
  ;[1 1 1] Target Perception Updated
  (bind _returnvalue (Class|AIPerceptionSystem|GetSenseClassforStimulus Stimulus))
  (if (== _returnvalue "/Script/AIModule.AISense_Sight")
    (if (and (Actor|ActorHasTag Actor (Variables|Default|GetTag)) (Utilities|Struct|BreakAIStimulus Stimulus))
      (Utilities|Time|ClearandInvalidateTimerbyHandle (Variables|Default|GetEnemy%20Timer)) ; Has Line of Sight
      (AI|Components|Blackboard|SetValueasBool _blackboard (Variables|Default|GetHasLineOfSight) true)
      (AI|Components|Blackboard|SetValueasObject _blackboard (Variables|Default|GetEnemyActor) Actor)
      (else
        (bind _returnvalue_2 (Utilities|Time|SetTimerbyEvent (delegate Custom|StartEnemyTimer) (Variables|Default|GetLineOfSightTimer)))
        (Variables|Default|SetEnemy%20Timer _returnvalue_2)))
    (else
      (CallFunction|HandleSoundSense Stimulus))))

(event Custom|StartEnemyTimer
  (bind _blackboard (Variables|Default|GetBlackboard))
  ;[1 1 1] Target Perception Updated
  (AI|Components|Blackboard|SetValueasBool _blackboard (Variables|Default|GetHasLineOfSight) false)
  (AI|Components|Blackboard|SetValueasObject _blackboard (Variables|Default|GetEnemyActor) 0))

(event EventPossess
  (params (PossessedPawn :type Pawn%20Object%20Reference))
  ;[1 1 1] On Possess
  (Variables|Default|SetAttachedPawn PossessedPawn) ; Save a reference to the attached pawn
  (AI|RunBehaviorTree "/Game/Blueprints/Enemies/BasicZombie/BT_BasicZombie.BT_BasicZombie") ; Run the behavior Tree
  (AI|Components|Blackboard|SetValueasBool (Variables|Default|GetBlackboard) (Variables|Default|GetIsAttacking) false) ; Initialize isAttacking to false
)

(fn ConstructionScript)

(fn HandleSoundSense
  (params (Stimulus :type AI%20Stimulus%20Structure%20%28by%20ref%29))
  (bind _returnvalue (Class|AIPerceptionSystem|GetSenseClassforStimulus Stimulus))
  (if (== _returnvalue "/Script/AIModule.AISense_Hearing")
    (AI|Components|Blackboard|SetValueasVector (Variables|Default|GetBlackboard) (Utilities|Name|MakeLiteralName "PatrolLocation") (.StimulusLocation (Utilities|Struct|BreakAIStimulus Stimulus)))))