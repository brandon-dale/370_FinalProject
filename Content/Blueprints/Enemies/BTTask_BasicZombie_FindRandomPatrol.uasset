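; Behavior tree task that picks a random patrol destination for the basic zombie.
; It sets the zombie's walk speed to the patrol speed, then writes a random reachable point within a radius of the pawn to the patrol location Blackboard key.
; If no point is found, it stores the pawn's current location and still succeeds, failing only when the pawn is not a BP_BasicZombie.
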(event EventReceiveExecuteAI
  (params (OwnerController :type AI%20Controller%20Object%20Reference) (ControlledPawn :type Pawn%20Object%20Reference))
  (bind _returnvalue (Transformation|GetActorLocation ControlledPawn))
  (bind _radius (Variables|Default|GetRadius))
  (bind (_randomlocation _returnvalue_2) (AI|Navigation|GetRandomReachablePointinRadius _returnvalue _radius 0 0))
  (bind _asbp_basic_zombie (Utilities|Casting|CastToBP_BasicZombie ControlledPawn)
    (:then
      (Default|UpdateWalkSpeed _asbp_basic_zombie (Variables|Default|GetPatrol%20Speed))
      (if _returnvalue_2
        (AI|BehaviorTree|SetBlackboardValueasVector (Variables|Default|GetPatrolLocation) _randomlocation)
        (else
          (AI|BehaviorTree|SetBlackboardValueasVector (Variables|Default|GetPatrolLocation) _returnvalue)))
      (AI|BehaviorTree|FinishExecute true))
    (:CastFailed
      (AI|BehaviorTree|FinishExecute false))))