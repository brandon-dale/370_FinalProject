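; Behavior tree task for the basic zombie that triggers a turn and clears the took-damage flag.
; It sets a target vector from either the player pawn's location or a blackboard location, depending on FacePlayer.
; RotateTowards on BP_BasicZombie receives a zero vector, not that target.
; The task then resets the TookDamage key and finishes successfully at once, without waiting for rotation.
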(event EventReceiveExecuteAI
  (params (OwnerController :type AI%20Controller%20Object%20Reference) (ControlledPawn :type Pawn%20Object%20Reference))
  (if (Variables|Default|GetFace%20Player)
    (Variables|Default|Settarget%20vector (Transformation|GetActorLocation (Game|Player|GetPlayerPawn 0)))
    (else
      (Variables|Default|Settarget%20vector (Class|BTFunctionLibrary|GetBlackboardValueasVector (Variables|Default|GetTarget%20Location%20BB%20Key)))))
  (bind _asbp_basic_zombie (Utilities|Casting|CastToBP_BasicZombie ControlledPawn)
    (:then
      (Default|RotateTowards _asbp_basic_zombie "0, 0, 0"))
    (:CastFailed
      _))
  (AI|Components|Blackboard|SetValueasBool (AI|GetBlackboard ControlledPawn) (Variables|Default|GetTookDamage%20Key) false)
  (AI|BehaviorTree|FinishExecute true))