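; CashDrop is a cash pickup that awards the player points when interacted with.
; Tick spins the actor around its local yaw axis at a rate set by the Rotation variable, scaled by delta time.
; The Interact event casts player pawn 0 to BP_FirstPersonCharacter, adds a fixed amount to its Points, destroys the pickup and plays a 2D cash sound.
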(event EventBeginPlay)

(event Collision|EventActorBeginOverlap
  (params (OtherActor :type Actor%20Object%20Reference)))

(event EventTick
  (params (DeltaSeconds :type Float%20%28single-precision%29))
  (Transformation|AddActorLocalRotation (Math|Rotator|MakeRotator 0.0 0.0 (* (Variables|Default|Getrotation) DeltaSeconds)) false false))

(event EventInteract
  (bind _asbp_first_person_character (Utilities|Casting|CastToBP_FirstPersonCharacter (Game|Player|GetPlayerPawn 0)))
  (Variables|/Game/FirstPerson/Blueprints/BP_FirstPersonCharacter.BP_FirstPersonCharacter_C|Setpoints _asbp_first_person_character (+ (Variables|/Game/FirstPerson/Blueprints/BP_FirstPersonCharacter.BP_FirstPersonCharacter_C|Getpoints _asbp_first_person_character) 100))
  (Actor|DestroyActor)
  (Audio|PlaySound2D "/Game/Blueprints/Pickups/sounds/cashpickup.cashpickup" 1.0 1.0 0.0 0 0))

(fn ConstructionScript)